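; Spawnable coin pickup that awards a point when a CharacterSphere overlaps its Icon component.
; A DoOnce limits collection to one overlap, which increments the character's Score, sets BeingDestroyed and destroys the coin after a short delay.
; It also returns its GridIndex to the AvailableGrids list of the first Grid actor, found at BeginPlay.
; An unconnected CharacterSphereBP cast path remains in the graph and never runs.
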(event OnComponentBeginOverlap(Icon)
  (params (OverlappedComponent :type Primitive%20Component%20Object%20Reference) (OtherActor :type Actor%20Object%20Reference) (OtherComp :type Primitive%20Component%20Object%20Reference) (OtherBodyIndex :type Integer) (bFromSweep :type Boolean) (SweepResult :type Hit%20Result%20Structure%20%28by%20ref%29))
  (bind _ascharacter_sphere (Utilities|Casting|CastToCharacterSphere OtherActor))
  (Utilities|FlowControl|DoOnce false
    (:Completed
      (Variables|/Script/MINIGAME.CharacterSphere|SetScore _ascharacter_sphere (+ (Variables|/Script/MINIGAME.CharacterSphere|GetScore _ascharacter_sphere) 1.0))
      (Variables|Default|SetBeingDestroyed true)
      (Utilities|Array|Add (Variables|/Game/Blueprints/Grid/Grid.Grid_C|GetAvailableGrids (Variables|Default|GetGrid)) (Variables|Default|GetGridIndex))
      (Utilities|FlowControl|Delay 1.0)
      (Actor|DestroyActor))))

(event EventBeginPlay
  (|CallParentFunction)
  (bind _outactors (Actor|GetAllActorsOfClass "/Game/Blueprints/Grid/Grid.Grid_C"))
  (Variables|Default|SetGrid (Utilities|Array|Get(acopy) _outactors)))

(event Collision|EventActorBeginOverlap
  (params (OtherActor :type Actor%20Object%20Reference))
  (|CallParentFunction OtherActor))

(event EventTick
  (params (DeltaSeconds :type Float%20%28single-precision%29))
  (|CallParentFunction DeltaSeconds) ; This node is disabled and will not be called.\nDrag off pins to build functionality.
)

(fn ConstructionScript
  (|CallParentFunction))