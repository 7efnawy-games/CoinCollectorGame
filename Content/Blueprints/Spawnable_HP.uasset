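; Health pickup actor that restores a fixed amount of the player sphere character's health, capped at the maximum.
; Overlapping the Icon triggers a one-shot heal, returns the pickup's index to the Grid actor's available spots, flags BeingDestroyed and destroys the actor after a short delay.
; The Grid is found in the level on BeginPlay, and the construction script rotates the icon.
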(event OnComponentBeginOverlap(Icon)
  (params (OverlappedComponent :type Primitive%20Component%20Object%20Reference) (OtherActor :type Actor%20Object%20Reference) (OtherComp :type Primitive%20Component%20Object%20Reference) (OtherBodyIndex :type Integer) (bFromSweep :type Boolean) (SweepResult :type Hit%20Result%20Structure%20%28by%20ref%29))
  (bind _ascharacter_sphere_bp (Utilities|Casting|CastToCharacterSphereBP OtherActor))
  (bind _output_get (Variables|Default|SetChar _ascharacter_sphere_bp))
  (if (Utilities|IsValid _output_get)
    (Utilities|FlowControl|DoOnce false
      (:Completed
        (Variables|/Script/MINIGAME.CharacterSphere|SetHealth _ascharacter_sphere_bp (Math|Float|Clamp(Float) (+ (Variables|/Script/MINIGAME.CharacterSphere|GetHealth _output_get) 2e+01) 0.0 1e+02))
        (Utilities|Array|Add (Variables|/Game/Blueprints/Grid/Grid.Grid_C|GetAvailableGrids (Variables|Default|GetGrid)) (Variables|Default|GetGridIndex))
        (Variables|Default|SetBeingDestroyed true)
        (Utilities|FlowControl|Delay 1.0)
        (Actor|DestroyActor)))))

(event Collision|EventActorBeginOverlap
  (params (OtherActor :type Actor%20Object%20Reference))
  (|CallParentFunction OtherActor) ; This node is disabled and will not be called.\nDrag off pins to build functionality.
)

(event EventTick
  (params (DeltaSeconds :type Float%20%28single-precision%29))
  (|CallParentFunction DeltaSeconds) ; This node is disabled and will not be called.\nDrag off pins to build functionality.
)

(event EventBeginPlay
  (bind _outactors (Actor|GetAllActorsOfClass "/Game/Blueprints/Grid/Grid.Grid_C"))
  (Variables|Default|SetGrid (Utilities|Array|Get(acopy) _outactors)))

(fn ConstructionScript
  (|CallParentFunction)
  (Transformation|AddRelativeRotation (Variables|Default|GetIcon) "90.000000, 0, 0" false false))