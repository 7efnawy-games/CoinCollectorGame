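; Health pickup actor that restores health to the player's CharacterSphereBP on overlap.
; When the Icon component overlaps that character, it adds a fixed amount to Health, clamped to the valid range.
; It then sets a BeingDestroyed flag and destroys itself after a short delay, with no guard against repeat overlaps during that delay.
; The construction script applies a rotation offset to the Icon.
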(event OnComponentBeginOverlap(Icon)
  (params (OverlappedComponent :type Primitive%20Component%20Object%20Reference) (OtherActor :type Actor%20Object%20Reference) (OtherComp :type Primitive%20Component%20Object%20Reference) (OtherBodyIndex :type Integer) (bFromSweep :type Boolean) (SweepResult :type Hit%20Result%20Structure%20%28by%20ref%29))
  (bind _ascharacter_sphere_bp (Utilities|Casting|CastToCharacterSphereBP OtherActor))
  (if (Utilities|IsValid _ascharacter_sphere_bp)
    (Variables|/Script/MINIGAME.CharacterSphere|SetHealth _ascharacter_sphere_bp (Math|Float|Clamp(Float) (+ (Variables|/Script/MINIGAME.CharacterSphere|GetHealth _ascharacter_sphere_bp) 2e+01) 0.0 1e+02))
    (Variables|Default|SetBeingDestroyed true)
    (Utilities|FlowControl|Delay 1.0)
    (Actor|DestroyActor)))

(event EventBeginPlay)

(event Collision|EventActorBeginOverlap
  (params (OtherActor :type Actor%20Object%20Reference)))

(event EventTick
  (params (DeltaSeconds :type Float%20%28single-precision%29)))

(fn ConstructionScript
  (Transformation|AddRelativeRotation (Variables|Default|GetIcon) "90.000000, 0,0.000000" false false))