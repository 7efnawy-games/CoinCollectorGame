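; Spawnable pickup-style actor with an Icon component that spins around yaw every Tick at a rate set by Frequency.
; When BeingDestroyed is set, the icon also rises by a fixed step each frame, independent of delta time.
; Collection logic that adds score to CharacterSphereBP, sets that flag and destroys the actor after a delay is unwired, and the Icon overlap event does nothing.
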(event OnComponentBeginOverlap(Icon)
  (params (OverlappedComponent :type Primitive%20Component%20Object%20Reference) (OtherActor :type Actor%20Object%20Reference) (OtherComp :type Primitive%20Component%20Object%20Reference) (OtherBodyIndex :type Integer) (bFromSweep :type Boolean) (SweepResult :type Hit%20Result%20Structure%20%28by%20ref%29)))

(event EventBeginPlay
  (|CallParentFunction))

(event Collision|EventActorBeginOverlap
  (params (OtherActor :type Actor%20Object%20Reference)))

(event EventTick
  (params (DeltaSeconds :type Float%20%28single-precision%29))
  (bind _frequency (Variables|Default|GetFrequency))
  (bind _icon (Variables|Default|GetIcon))
  (bind _returnvalue (* _frequency 3.6e+02))
  (bind _returnvalue_2 (Math|Float|Truncate _returnvalue))
  (bind _returnvalue_3 (Math|Conversions|ToFloat(Integer) _returnvalue_2))
  (bind _returnvalue_4 (* DeltaSeconds _returnvalue_3))
  (if (Variables|Default|GetBeingDestroyed)
    (Transformation|AddRelativeRotation _icon (Math|Rotator|MakeRotator 0.0 0.0 _returnvalue_4) false false)
    (Transformation|AddRelativeLocation _icon (Math|Vector|MakeVector 0.0 0.0 1e+01) false false)
    (else
      (Transformation|AddRelativeRotation (Variables|Default|GetIcon) (Math|Rotator|MakeRotator 0.0 0.0 _returnvalue_4) false false))))

(fn ConstructionScript)